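; SpawnSoundObject_BP is a construction-time spawner that places child actors, apparently sound objects, inside a box area.
; Its construction script stores the relative transforms of three spawn point components, then adds two child actor components at random points within the SOArea box.
; The stored spawn points are not used for placement in this graph, and the event graph has no active logic.
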(event EventBeginPlay)

(event Collision|EventActorBeginOverlap
  (params (OtherActor :type Actor%20Object%20Reference)))

(event EventTick
  (params (DeltaSeconds :type Float%20%28single-precision%29)))

(fn ConstructionScript
  (CallFunction|SpawnObjectPoints)
  (CallFunction|SpawnSoundObj))

(fn SpawnSoundObj
  (bind _soarea (Variables|Default|GetSOArea))
  (for _index (range 0 1)
    (AddComponent|AddChildActorComponent false (Math|Conversions|ToTransform(Vector) (Math|Random|RandomPointinBoundingBox (Variables|/Script/Engine.SceneComponent|GetRelativeLocation _soarea) (Variables|/Script/Engine.BoxComponent|GetBoxExtent _soarea))))))

(fn SpawnObjectPoints
  (Variables|Default|SetSpawnPoints (Utilities|Array|MakeArray (Transformation|GetRelativeTransform (Variables|Default|GetSpawnPoint)) (Transformation|GetRelativeTransform (Variables|Default|GetSpawnPoint1)) (Transformation|GetRelativeTransform (Variables|Default|GetSpawnPoint2)))))