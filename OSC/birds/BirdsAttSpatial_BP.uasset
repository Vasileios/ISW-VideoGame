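; Bird spatial-sound actor (by path and name) that sends OSC triggers to SC when its box overlap begins or ends.
; Overlaps also toggle a point light and particle system, and ManageIpPortOsc registers the send target.
; If ActivePlanet is set, a timeline moves the actor along OrbitReference's spline from BeginPlay.
; Distance-based amplitude and dot-product panning graphs are present but disconnected, so Tick sends nothing.
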(event OnComponentBeginOverlap(Box)
  (params (OverlappedComponent :type Primitive%20Component%20Object%20Reference) (OtherActor :type Actor%20Object%20Reference) (OtherComp :type Primitive%20Component%20Object%20Reference) (OtherBodyIndex :type Integer) (bFromSweep :type Boolean) (SweepResult :type Hit%20Result%20Structure%20%28by%20ref%29))
  (bind _particlesystem (Variables|Default|GetParticleSystem))
  (bind _pointlight (Variables|Default|GetPointLight))
  ;[0.151 0.3022 1] SendOSC to SC. Events Overlap Function
  (Variables|Default|Settrigger1 (Variables|Default|Gettrigger1))
  (CallFunction|EventBeginOverlapOscSend "/Game/FirstPersonCPP/Blueprints/FirstPersonCharacter.FirstPersonCharacter_C")
  (Rendering|SetVisibility _pointlight true false)
  (Rendering|Components|Light|SetIntensity _pointlight (Variables|Default|GetLightIntensity))
  (Components|Activation|SetActive _particlesystem true false)
  (Rendering|SetVisibility _particlesystem true false))

(event OnComponentEndOverlap(Box)
  (params (OverlappedComponent :type Primitive%20Component%20Object%20Reference) (OtherActor :type Actor%20Object%20Reference) (OtherComp :type Primitive%20Component%20Object%20Reference) (OtherBodyIndex :type Integer))
  (bind _particlesystem (Variables|Default|GetParticleSystem))
  ;[0.151 0.3022 1] SendOSC to SC. Events Overlap Function
  (CallFunction|EventEndOverlapOscSend "/Game/FirstPersonCPP/Blueprints/FirstPersonCharacter.FirstPersonCharacter_C")
  (Rendering|SetVisibility (Variables|Default|GetPointLight) false false)
  (Components|Activation|SetActive _particlesystem false false)
  (Rendering|SetVisibility _particlesystem false false))

(event Custom|Event%20OSCFunc
  ;[0.151 0.3022 1] SendOSC to SC. Events Overlap Function
)

(event Custom|EventSendOSC
  ;[1 0.5426 0.0514] CalculateDistance between player and object's attenuation radius
)

(event Custom|EvalOrbit
  (bind _orbitreference (Variables|Default|GetorbitReference))
  (bind _spline (Variables|/Game/OSC/birds/ObjectOrbit_BP.ObjectOrbit_BP_C|GetSpline _orbitreference))
  ;[1 1 1] Evaluate orbit
  (Components|Timeline|SetPlayRate (Variables|Default|GetPlanetMover) (/ 1.0 (Variables|Default|Getduration)))
  (Components|Timeline|SetNewTime (Variables|Default|GetPlanetMover) (Variables|Default|GetplanetStartOffset))
  (bind _alpha (Timeline|PlanetMover Play)
    (:Update
      (Variables|Default|SetAlpha _alpha)
      (Transformation|SetActorLocationAndRotation (Spline|GetLocationatDistanceAlongSpline _spline (Math|Float|Lerp 0.0 (Spline|GetSplineLength _spline) (Variables|Default|GetAlpha)) "World") (Spline|GetRotationatDistanceAlongSpline _spline (Math|Float|Lerp 0.0 (Spline|GetSplineLength _spline) (Variables|Default|GetAlpha)) "World")))))

(event Collision|EventActorBeginOverlap
  (params (OtherActor :type Actor%20Object%20Reference)))

(event EventTick
  (params (DeltaSeconds :type Float%20%28single-precision%29))
  ;[0.3439 0 1] Event Tick
  (bind _output_get (Variables|Default|SetisOverlap? true))
  (if _output_get
    (Utilities|FlowControl|Sequence)))

(event EventBeginPlay
  ;[1 1 1] Evaluate orbit
  (if (Variables|Default|GetactivePlanet)
    (CallFunction|EvalOrbit)))

(fn ConstructionScript)

(fn EventBeginOverlapOscSend
  (params (PlayerCharacter :type Actor%20Class%20Reference))
  ;[1 1 1] Send OSC when begin overlap
  (Utilities|FlowControl|Sequence
    (:then_0
      (Utilities|FlowControl|DoOnce false
        (:Completed
          (Utilities|Casting|CastToFirstPersonCharacterSmallGl (Game|GetPlayerCharacter 0))
          (bind _output_get (Variables|Default|Settrigger1 (Variables|Default|Gettrigger1)))
          (CallFunction|ManageIpPortOsc)
          (Utilities|Time|SetTimerbyEvent (EventDispatchers|CreateEvent :!event Custom|EventSendOSC) 1.0)
          (Class|OscFunctionLibrary|SendOsc (Variables|Default|Getaddress_trigger) (Class|OscFunctionLibrary|PushInt 0 _output_get) -1)
          (Variables|Default|SetisOverlap? true)
          (return))))))

(fn EventEndOverlapOscSend
  (params (PlayerCharacter :type Actor%20Class%20Reference))
  ;[1 1 1] Send OSC when begin overlap
  (Utilities|FlowControl|DoOnce false
    (:Completed
      (Utilities|Casting|CastToFirstPersonCharacterSmallGl (Game|GetPlayerCharacter 0))
      (bind _output_get (Variables|Default|SettriggerOut 1))
      (CallFunction|ManageIpPortOsc)
      (Utilities|Time|SetTimerbyEvent (EventDispatchers|CreateEvent :!event Custom|EventSendOSC) 1.0)
      (Class|OscFunctionLibrary|SendOsc (Variables|Default|Getaddress_trigger) (Class|OscFunctionLibrary|PushInt 0 _output_get) -1))))

(fn ManageIpPortOsc
  (Variables|Default|SetbisSet (not (Variables|Default|GetbisSet)))
  (Class|OscFunctionLibrary|AddSendOscTarget (Variables|Default|GetipPort2))
  (Class|OscFunctionLibrary|AddSendOscTarget (Variables|Default|GetipPort2))
  (Utilities|Time|SetTimerbyEvent (EventDispatchers|CreateEvent :!event Custom|EventSendOSC) 1.0))