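; ObjectOrbit_BP builds a circular orbit path as a spline sized by SplineRadius; no movement along it is implemented here.
; The Construction Script clears the spline and places four local-space points on the X and Y axes.
; It then sets each point's tangent perpendicular to its axis, scaled by the radius and a constant meant to approximate a circle with Bezier curves.
; The event graph holds only disabled stub events.
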(event EventBeginPlay)

(event Collision|EventActorBeginOverlap
  (params (OtherActor :type Actor%20Object%20Reference)))

(event EventTick
  (params (DeltaSeconds :type Float%20%28single-precision%29)))

(fn ConstructionScript
  (bind _spline (Variables|Default|GetSpline))
  (bind _splineradius (Variables|Default|GetsplineRadius))
  (bind _spline_2 (Variables|Default|GetSpline))
  (bind _splineradius_2 (Variables|Default|GetsplineRadius))
  (bind _spline_3 (Variables|Default|GetSpline))
  (bind _returnvalue (* _splineradius -1.0))
  ;[0 0.07301 1] Create Circle spline
  (Spline|ClearSplinePoints _spline_2 true)
  (Spline|AddSplinePoint _spline_2 (Math|Vector|MakeVector _splineradius_2 0.0 0.0) "Local" true)
  (Spline|AddSplinePoint _spline_2 (Math|Vector|MakeVector 0.0 _splineradius_2 0.0) "Local" true)
  (Spline|AddSplinePoint _spline (Math|Vector|MakeVector _returnvalue 0.0 0.0) "Local" true)
  (Spline|AddSplinePoint _spline (Math|Vector|MakeVector 0.0 _returnvalue 0.0) "Local" true)
  (Variables|Default|SetcircleConstant (+ (Math|Conversions|ToFloat(Integer) (|((4*(8-1))/3))) 1.0))
  (for _index (range 0 (Spline|GetNumberOfSplinePoints (Variables|Default|GetSpline)))
    (switch int _index
      (:0
        (Spline|SetTangentatSplinePoint _spline_3 _index (Math|Vector|MakeVector 0.0 (* (* (Variables|Default|GetcircleConstant) (Variables|Default|GetsplineRadius)) 1.0) 0.0) "Local" true))
      (:1
        (Spline|SetTangentatSplinePoint _spline_3 _index (Math|Vector|MakeVector (* (* (Variables|Default|GetcircleConstant) (Variables|Default|GetsplineRadius)) -1.0) 0.0 0.0) "Local" true))
      (:2
        (Spline|SetTangentatSplinePoint _spline_3 _index (Math|Vector|MakeVector 0.0 (* (* (Variables|Default|GetcircleConstant) (Variables|Default|GetsplineRadius)) -1.0) 0.0) "Local" true))
      (:3
        (Spline|SetTangentatSplinePoint _spline_3 _index (Math|Vector|MakeVector (* (* (Variables|Default|GetcircleConstant) (Variables|Default|GetsplineRadius)) 1.0) 0.0 0.0) "Local" true)))))